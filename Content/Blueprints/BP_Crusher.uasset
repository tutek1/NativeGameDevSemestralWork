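; BP_Crusher is a crusher actor whose Cube moves continuously up and down between two height limits.
; Each Tick offsets the Cube's relative Z by delta time, Speed and SpeedModifier, with direction chosen by IsGoingUp.
; The flag flips when world Z passes MinZ or MaxZ, and its name is inverted, since true moves the Cube in negative Z.
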(event EventTick
  (params (DeltaSeconds :type Float%20%28single-precision%29))
  (bind _speedmodifier (Variables|Default|GetSpeedModifier))
  (bind _speed (Variables|Default|GetSpeed))
  (bind _cube (Variables|Default|GetCube))
  (bind _returnvalue (* _speed _speedmodifier))
  (bind _returnvalue_2 (* DeltaSeconds _returnvalue))
  ;[1 1 1] Move the crusher up or down
  (if (Variables|Default|GetIsGoingUp)
    (Transformation|AddRelativeLocation _cube (Math|Vector|MakeVector 0.0 0.0 (* _returnvalue_2 -1.0)) false false)
    (else
      (Transformation|AddRelativeLocation _cube (Math|Vector|MakeVector 0.0 0.0 _returnvalue_2) false false)))
  ;[1 1 1] Check if the direction needs to be changed based on the limits
  (if (< (.z (Transformation|GetWorldLocation (Variables|Default|GetCube))) (Variables|Default|GetMinZ))
    (Variables|Default|SetIsGoingUp false)
    (elif (> (.z (Transformation|GetWorldLocation (Variables|Default|GetCube))) (Variables|Default|GetMaxZ))
      (Variables|Default|SetIsGoingUp true))))

(fn ConstructionScript)