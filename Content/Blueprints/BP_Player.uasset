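; Player character with tank-style turn and move controls that teleports back to its start position when hit by a Crusher-tagged actor.
; One ability input triggers either levitation, which zeroes gravity at a set height, or, failing that, a slowdown of all BP_Crusher actors.
; Each ability runs for AbilityDuration, with a duration-scaled timeline filling the progress bar of a widget created on BeginPlay.
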(event EventBeginPlay
  ;[1 1 1] Get the position to reset to
  (Variables|Default|SetStartPosition (Transformation|GetWorldLocation (Variables|Transformation|GetRootComponent)))
  ;[1 1 1] Create the visual effect of timeslow and hide it
  (bind _returnvalue (UserInterface|CreateWidget "/Game/Blueprints/BP_TimeSlow_Effect.BP_TimeSlow_Effect_C"))
  (bind _output_get (Variables|Default|SetTimeSlowUI _returnvalue))
  (UserInterface|Viewport|AddtoViewport _output_get 0)
  (Widget|SetVisibility _output_get "Hidden")
  ;[1 1 1] Create the visual effect of levitate and hide it
  (bind _returnvalue_2 (UserInterface|CreateWidget "/Game/Blueprints/BP_Levitate_Effect.BP_Levitate_Effect_C"))
  (bind _output_get_2 (Variables|Default|SetLevitateUI _returnvalue_2))
  (UserInterface|Viewport|AddtoViewport _output_get_2 0)
  (Widget|SetVisibility _output_get_2 "Hidden"))

(event Collision|EventHit
  (params (MyComp :type Primitive%20Component%20Object%20Reference) (Other :type Actor%20Object%20Reference) (OtherComp :type Primitive%20Component%20Object%20Reference) (bSelfMoved :type Boolean) (HitLocation :type Vector :default "0, 0, 0") (HitNormal :type Vector :default "0, 0, 0") (NormalImpulse :type Vector :default "0, 0, 0") (Hit :type Hit%20Result%20Structure%20%28by%20ref%29))
  ;[1 1 1] Crusher reset detection
  (if (Actor|ActorHasTag Other "Crusher")
    (Transformation|SetWorldLocation (Variables|Transformation|GetRootComponent) (Variables|Default|GetStartPosition) false false)))

(event Input|ActionEvents|InputActionAbility
  (params (Key :type Key%20Structure :default "None"))
  (bind _rootcomponent (Variables|Transformation|GetRootComponent))
  (bind _abilityduration (Variables|Default|GetAbilityDuration))
  (bind _timeslowui (Variables|Default|GetTimeSlowUI))
  (bind _abilityduration_2 (Variables|Default|GetAbilityDuration))
  (bind _levitateui (Variables|Default|GetLevitateUI))
  (bind _returnvalue (Transformation|GetWorldLocation _rootcomponent))
  ;[1 1 1] Handle Ability Press
  (:Pressed
    (if (not (Variables|Default|GetIsAbilityActive))
      (if (Variables|Default|GetHasLevitation)
        ;[1 1 1] Levitate Ability
        (Variables|Default|SetIsAbilityActive true)
        (Variables|/Script/Engine.CharacterMovementComponent|SetGravityScale (Variables|Character|GetCharacterMovement) 0.0)
        (Transformation|SetWorldLocation _rootcomponent (Math|Vector|MakeVector (.x _returnvalue) (.y _returnvalue) (Variables|Default|GetLevitationHeight)) false false)
        (Widget|SetVisibility _levitateui "Visible")
        (Components|Timeline|SetPlayRate (Variables|Default|GetTimeline_0) (/ 1.0 _abilityduration))
        (bind _percentage (Timeline|Timeline_0 PlayFromStart)
          (:Update
            (Progress|SetPercent (Variables|/Game/Blueprints/BP_Levitate_Effect.BP_Levitate_Effect_C|GetProgressBar _levitateui) _percentage)
            (Utilities|FlowControl|Delay (Variables|Default|GetAbilityDuration))
            (Variables|Default|SetIsAbilityActive false)
            (Variables|/Script/Engine.CharacterMovementComponent|SetGravityScale (Variables|Character|GetCharacterMovement) 1.0)
            (Widget|SetVisibility _levitateui "Hidden")))
        (elif (Variables|Default|GetHasTimeSlow)
          ;[1 1 1] Time Stop Ability (for all crushers)
          (Variables|Default|SetIsAbilityActive true)
          (bind _outactors (Actor|GetAllActorsOfClass "/Game/Blueprints/BP_Crusher.BP_Crusher_C"))
          (for _array_element _outactors
            (Variables|/Game/Blueprints/BP_Crusher.BP_Crusher_C|SetSpeedModifier _array_element (Variables|Default|GetTimeSlowModifier))
            (Widget|SetVisibility _timeslowui "Visible")
            (Components|Timeline|SetPlayRate (Variables|Default|GetTimeline) (/ 1.0 _abilityduration_2))
            (bind _percentage_2 (Timeline|Timeline PlayFromStart)
              (:Update
                (Progress|SetPercent (Variables|/Game/Blueprints/BP_TimeSlow_Effect.BP_TimeSlow_Effect_C|GetProgressBar _timeslowui) _percentage_2))))
          (Utilities|FlowControl|Delay (Variables|Default|GetAbilityDuration))
          (Variables|Default|SetIsAbilityActive false)
          (bind _outactors_2 (Actor|GetAllActorsOfClass "/Game/Blueprints/BP_Crusher.BP_Crusher_C"))
          (for _array_element_2 _outactors_2
            (Variables|/Game/Blueprints/BP_Crusher.BP_Crusher_C|SetSpeedModifier _array_element_2 1.0)
            (Widget|SetVisibility (Variables|Default|GetTimeSlowUI) "Hidden")))))))

(event Input|ActionEvents|InputActionTurnRight
  (params (Key :type Key%20Structure :default "None"))
  ;[1 1 1] Movement and Turning
  (:Pressed
    (Class|Actor|AddActorWorldRotation (Math|Rotator|MakeRotator 0.0 0.0 (Variables|Default|GetTurnSpeed)))))

(event Input|ActionEvents|InputActionTurnLeft
  (params (Key :type Key%20Structure :default "None"))
  ;[1 1 1] Movement and Turning
  (:Pressed
    (Class|Actor|AddActorWorldRotation (Math|Rotator|MakeRotator 0.0 0.0 (* -1.0 (Variables|Default|GetTurnSpeed))))))

(event Input|AxisEvents|InputAxisMove
  (params (AxisValue :type Float%20%28single-precision%29))
  ;[1 1 1] Movement and Turning
  (Pawn|Input|AddMovementInput (Math|Vector|GetForwardVector (Variables|Collision|GetCapsuleComponent)) (* AxisValue (Variables|Default|GetMoveSpeed)) false))

(fn ConstructionScript)